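; Trigger actor that flashes a turn indicator on the W_Turns HUD widget when an actor overlaps it.
; On overlap it finds every W_Turns widget and switches on TurnType, which covers left and right variants of grades 1–6, SQ and HP.
; Each case feeds the matching widget element into its own identical sub-graph, which shows it for two seconds, then hides it.
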(event EventBeginPlay)

(event Collision|EventActorBeginOverlap
  (params (OtherActor :type Actor%20Object%20Reference))
  (bind _foundwidgets (Widget|GetAllWidgetsOfClass "/Game/UI/W_Turns.W_Turns_C" false))
  (for _array_element _foundwidgets
    (switch string (Variables|Default|GetTurnType) ; Turn order HP,SQ,1,2,3,4,5,6,7
      (:1L
        (Utilities|String|Left (Variables|/Game/UI/W_Turns.W_Turns_C|GetL1 _array_element)))
      (:2L
        (|left_2 (Variables|/Game/UI/W_Turns.W_Turns_C|GetL2 _array_element)))
      (:3L
        (|left_3 (Variables|/Game/UI/W_Turns.W_Turns_C|GetL3 _array_element)))
      (:4L
        (|left_4 (Variables|/Game/UI/W_Turns.W_Turns_C|GetL4 _array_element)))
      (:5L
        (|left_5 (Variables|/Game/UI/W_Turns.W_Turns_C|GetL5 _array_element)))
      (:6L
        (|left_6 (Variables|/Game/UI/W_Turns.W_Turns_C|GetL6 _array_element)))
      (:SQ_L
        (|left_sq (Variables|/Game/UI/W_Turns.W_Turns_C|GetSQ_L _array_element)))
      (:HP_L
        (|left_hp (Variables|/Game/UI/W_Turns.W_Turns_C|GetHP_L _array_element)))
      (:1R
        (|right_1 (Variables|/Game/UI/W_Turns.W_Turns_C|GetR1 _array_element)))
      (:2R
        (|right_2 (Variables|/Game/UI/W_Turns.W_Turns_C|GetR2 _array_element)))
      (:3R
        (|right_3 (Variables|/Game/UI/W_Turns.W_Turns_C|GetR3 _array_element)))
      (:4R
        (|right_4 (Variables|/Game/UI/W_Turns.W_Turns_C|GetR4 _array_element)))
      (:5R
        (|right_5 (Variables|/Game/UI/W_Turns.W_Turns_C|GetR5 _array_element)))
      (:6R
        (|Right_6 (Variables|/Game/UI/W_Turns.W_Turns_C|GetR6 _array_element)))
      (:SQ_R
        (|Right_sq (Variables|/Game/UI/W_Turns.W_Turns_C|GetSQ_R _array_element)))
      (:HP_R
        (|Right_hp (Variables|/Game/UI/W_Turns.W_Turns_C|GetHP_R _array_element))))))

(event EventTick
  (params (DeltaSeconds :type Float%20%28single-precision%29)))

(fn ConstructionScript)