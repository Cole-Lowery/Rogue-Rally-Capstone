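; BP_terrain is an actor that builds a procedural grass terrain mesh with collision, in both the construction script and BeginPlay.
; Generation lays out a vertex grid sized by XVert, YVert and CellSize, with height from summed 1D Perlin noise on each axis.
; It appends two triangles per cell to arrays it never clears, then creates the TerrainMesh section without normals or UVs.
; ShowDebug draws debug boxes and lines during generation.
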(event EventBeginPlay
  (CallFunction|Generation))

(event Collision|EventActorBeginOverlap
  (params (OtherActor :type Actor%20Object%20Reference)))

(event EventTick
  (params (DeltaSeconds :type Float%20%28single-precision%29)))

(fn ConstructionScript
  (CallFunction|Generation))

(fn Generation
  (bind _triangle (Variables|Default|GetTriangle))
  (bind _xvert (Variables|Default|GetXVert))
  (bind _triangle_2 (Variables|Default|GetTriangle))
  (bind _cellsize (Variables|Default|GetCellSize))
  (for _index (range 0 (- (Variables|Default|GetYVert) 1))
    (for _index_2 (range 0 (- (Variables|Default|GetXVert) 1))
      (Utilities|Array|Add (Variables|Default|GetVetices) (Math|Vector|MakeVector (* _cellsize _index_2) (* _index _cellsize) (* (+ (Class|KismetMathLibrary|PerlinNoise1D (+ (* _cellsize _index_2) 0.1)) (Class|KismetMathLibrary|PerlinNoise1D (+ (* _index _cellsize) 0.1))) 5e+03)))
      (if (Variables|Default|GetShowDebug)
        (Rendering|Debug|DrawDebugBox (Math|Vector|MakeVector (* _cellsize _index_2) (* _index _cellsize) 0.0) "2.000000,2.000000,2.000000" "(R=1.000000,G=0.000000,B=0.000000,A=1.000000)" "0, 0, 0" 1e+02 1e+02))))
  (for _index_3 (range 0 (- (Variables|Default|GetYVert) 2))
    (for _index_4 (range 0 (- (Variables|Default|GetXVert) 2))
      (Utilities|Array|Add _triangle_2 (+ _index_4 (* _index_3 _xvert)))
      (Utilities|Array|Add _triangle_2 (+ (+ _index_4 (* _index_3 _xvert)) _xvert))
      (Utilities|Array|Add _triangle_2 (+ (+ _index_4 (* _index_3 _xvert)) 1))
      (Utilities|Array|Add _triangle (+ (+ _index_4 (* _index_3 _xvert)) _xvert))
      (Utilities|Array|Add _triangle (+ (+ (+ _index_4 (* _index_3 _xvert)) _xvert) 1))
      (Utilities|Array|Add _triangle (+ (+ _index_4 (* _index_3 _xvert)) 1))
      (if (Variables|Default|GetShowDebug)
        (Rendering|Debug|DrawDebugLine (Utilities|Array|Get(acopy) (Variables|Default|GetVetices) (+ (+ _index_4 (* _index_3 _xvert)) 1)) (+ (Utilities|Array|Get(acopy) (Variables|Default|GetVetices) (+ (+ _index_4 (* _index_3 _xvert)) 1)) "0.000000,0.000000,10.000000") "(R=1.000000,G=0.000000,B=0.000000,A=1.000000)" 1e+02 2e+01))))
  (Class|ProceduralMeshComponent|CreateMeshSectionLinearColor (Variables|Default|GetTerrainMesh) 0 (Variables|Default|GetVetices) (Variables|Default|GetTriangle) 0 0 0 0 0 0 0 true false)
  (Rendering|Material|SetMaterial (Variables|Default|GetTerrainMesh) 0 "/Game/CountryRoads_Set01/DEMO/Ground_Textures/M_Grass_Landscape.M_Grass_Landscape"))