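; Procedural road generator that builds a wobbly spline road between Start and End actors in the construction script.
; It interpolates points at mesh-length spacing, offsetting them with a seeded stream whose range also uses unseeded random values.
; Spline mesh components are then added along each segment, sized near the mesh length.
; After each mesh is added, vertical line traces snap all road points onto the surface they hit.
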(event EventBeginPlay)

(event Collision|EventActorBeginOverlap
  (params (OtherActor :type Actor%20Object%20Reference)))

(event EventTick
  (params (DeltaSeconds :type Float%20%28single-precision%29)))

(fn ConstructionScript
  (CallFunction|NewFunction))

(fn NewFunction
  (bind _returnvalue (Math|Random|RandomFloat))
  (bind _meshlength (Variables|Default|GetMeshlength))
  (bind _road (Variables|Default|GetRoad))
  (bind _road_2 (Variables|Default|GetRoad))
  (bind _road_3 (Variables|Default|GetRoad))
  (bind _start (Variables|Default|GetStart))
  (bind _end (Variables|Default|GetEnd))
  (bind _maxwobble (Variables|Default|GetMaxWobble))
  (bind _returnvalue_2 (Transformation|GetActorTransform _start))
  (bind _returnvalue_3 (Transformation|GetActorTransform _end))
  (bind _returnvalue_4 (Math|Vector|Distance(Vector) (.location _returnvalue_2) (.location _returnvalue_3)))
  (bind _returnvalue_5 (/ _returnvalue_4 _meshlength))
  (Spline|ClearSplinePoints (Variables|Default|GetSpline) true)
  (Spline|ClearSplinePoints _road_3 true)
  (bind _output_get (Variables|Default|SetLocalStream (Math|Random|MakeRandomStream (Variables|Default|GetSeed))))
  (for _index (range 0 _returnvalue_5)
    (Spline|AddSplinePointatIndex (Variables|Default|GetRoad) (+ (* (Math|Random|RandomFloatinRangefromStream _output_get -1e+03 _returnvalue) (Math|Vector|MakeVector (* (* _maxwobble (Math|Random|RandomFloatinRangefromStream _output_get -1e+03 _returnvalue)) 0.01) (* (* _maxwobble (Math|Random|RandomFloatinRangefromStream _output_get -1e+03 _returnvalue)) 0.01) 0.0)) (Math|Vector|Lerp(Vector) (.location _returnvalue_2) (.location _returnvalue_3) (Math|Conversions|ToFloat(Integer) (/ _index (Math|Float|Ceil (Math|Conversions|ToFloat(Integer) _returnvalue_5)))))) _index "Local" true))
  (for _index_2 (range 0 (- (Spline|GetNumberOfSplinePoints _road_3) 2))
    (bind _output_get_2 (Variables|Default|SetCurSplineDis (Spline|GetDistanceAlongSplineatSplinePoint (Variables|Default|GetRoad) _index_2)))
    (bind _output_get_3 (Variables|Default|SetCurrSplinrLength (+ _output_get_2 (Spline|GetDistanceAlongSplineatSplinePoint (Variables|Default|GetRoad) (+ _index_2 1)))))
    (bind _output_get_4 (Variables|Default|SetNumSplineMeshes (/ _output_get_3 (Variables|Default|GetMeshlength))))
    (if (> _output_get_4 0)
      (bind _output_get_5 (Variables|Default|SetStrechMeshLeng (/ (Variables|Default|GetCurrSplinrLength) (Variables|Default|GetNumSplineMeshes))))
      (if (< _output_get_5 (* (Variables|Default|GetMeshlength) 1.5))
        _
        (else
          (Variables|Default|SetStrechMeshLeng (/ (Variables|Default|GetStrechMeshLeng) 2.0))
          (Variables|Default|SetNumSplineMeshes (* (Variables|Default|GetNumSplineMeshes) 2))))
      (for _index_3 (range 0 (- (Variables|Default|GetNumSplineMeshes) 1))
        (bind _returnvalue_6 (AddComponent|AddSplineMeshComponent false))
        (SplineMesh|SetStartandEnd _returnvalue_6 (Spline|GetLocationatDistanceAlongSpline _road_2 (+ (* _index_3 (Variables|Default|GetStrechMeshLeng)) (Variables|Default|GetCurSplineDis)) "Local") (Math|Vector|ClampVectorSize (Math|Conversions|ToVector(Float) (Class|SplineComponent|GetTimeatDistanceAlongSpline _road_2 (+ (* _index_3 (Variables|Default|GetStrechMeshLeng)) (Variables|Default|GetCurSplineDis)))) 0.0 (Variables|Default|GetStrechMeshLeng)) (Spline|GetLocationatDistanceAlongSpline _road (+ (* (+ _index_3 1) (Variables|Default|GetStrechMeshLeng)) (Variables|Default|GetCurSplineDis)) "Local") (Math|Vector|ClampVectorSize (Math|Conversions|ToVector(Float) (Class|SplineComponent|GetTimeatDistanceAlongSpline _road (+ (* (+ _index_3 1) (Variables|Default|GetStrechMeshLeng)) (Variables|Default|GetCurSplineDis)))) 0.0 (Variables|Default|GetStrechMeshLeng)) true :!class /Script/Engine.SplineMeshComponent)
        (Transformation|AttachComponentToComponent _returnvalue_6 (Variables|Default|GetRoad) "None" "KeepRelative" "KeepRelative" "KeepRelative" true)
        (CallFunction|NewFunction1)))))

(fn NewFunction1
  (bind _road (Variables|Default|GetRoad))
  (for _index (range 0 (- (Spline|GetNumberOfSplinePoints (Variables|Default|GetRoad)) 1))
    (bind _output_get (Variables|Default|SetStart_v (Math|Vector|MakeVector (.x (Spline|GetLocationatSplinePoint _road _index "World")) (.y (Spline|GetLocationatSplinePoint _road _index "World")) (+ (.z (Spline|GetLocationatSplinePoint _road _index "World")) 5e+03))))
    (bind _output_get_2 (Variables|Default|SetEnd_v (Math|Vector|MakeVector (.x (Spline|GetLocationatSplinePoint _road _index "World")) (.y (Spline|GetLocationatSplinePoint _road _index "World")) (- (.z (Spline|GetLocationatSplinePoint _road _index "World")) 5e+03))))
    (bind (_outhit _returnvalue) (Collision|LineTraceByChannel _output_get _output_get_2 "TraceTypeQuery1" false 0 "None"))
    (if _returnvalue
      (Spline|SetLocationatSplinePoint (Variables|Default|GetRoad) _index (.location _outhit) "World" true)))
  (Spline|UpdateSpline _road))