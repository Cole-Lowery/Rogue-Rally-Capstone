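; BP_Camera sets up the main menu when play begins.
; BeginPlay creates W_Main_Menu, adds it to the viewport and sets Game and UI input mode focused on it, then calls MenuMusic.
; MenuMusic picks a random integer to play one 2D track, with Running From The Future mapped to two outcomes, so it is twice as likely.
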(event EventBeginPlay
  (Utilities|FlowControl|Sequence
    (:then_0
      (bind _returnvalue (UserInterface|CreateWidget "/Game/UI/W_Main_Menu.W_Main_Menu_C"))
      (UserInterface|Viewport|AddtoViewport _returnvalue 0)
      (Input|SetInputModeGameandUI (Game|GetPlayerController 0) _returnvalue "DoNotLock" false false))
    (:then_1
      (CallFunction|MenuMusic))))

(event Collision|EventActorBeginOverlap
  (params (OtherActor :type Actor%20Object%20Reference)))

(event EventTick
  (params (DeltaSeconds :type Float%20%28single-precision%29)))

(fn ConstructionScript)

(fn MenuMusic
  (switch int (Math|Random|RandomIntegerinRange 0 9)
    (:Default
      (Audio|PlaySound2D "/Game/Music/25__Turn_Blue.25__Turn_Blue" 1.0 1.0 0.0 0 0))
    (:0
      (Audio|PlaySound2D "/Game/Music/04__Burning_Out.04__Burning_Out" 1.0 1.0 0.0 0 0))
    (:1
      (Audio|PlaySound2D "/Game/Music/07__Dose.07__Dose" 1.0 1.0 0.0 0 0))
    (:2
      (Audio|PlaySound2D "/Game/Music/11__I_Want_More.11__I_Want_More" 1.0 1.0 0.0 0 0))
    (:3
      (Audio|PlaySound2D "/Game/Music/12__Mechanical_World.12__Mechanical_World" 1.0 1.0 0.0 0 0))
    (:4
      (Audio|PlaySound2D "/Game/Music/18__Running_From_The_Future.18__Running_From_The_Future" 1.0 1.0 0.0 0 0))
    (:5
      (Audio|PlaySound2D "/Game/Music/18__Running_From_The_Future.18__Running_From_The_Future" 1.0 1.0 0.0 0 0))
    (:6
      (Audio|PlaySound2D "/Game/Music/19__Skywind.19__Skywind" 1.0 1.0 0.0 0 0))
    (:7
      (Audio|PlaySound2D "/Game/Music/20__Spit.20__Spit" 1.0 1.0 0.0 0 0))
    (:8
      (Audio|PlaySound2D "/Game/Music/21__Suicide_Mind.21__Suicide_Mind" 1.0 1.0 0.0 0 0))))